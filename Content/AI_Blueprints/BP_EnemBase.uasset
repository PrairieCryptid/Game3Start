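; BP_EnemBase is an AI enemy base with patrol, investigate, aggro and kick-attack behavior.
; Aggro and investigate events set state flags and swap the mesh to red or green debug-style materials, restoring the original material on exit.
; GetNextPatrolPointLocation steps along the PatrolRoute spline points, reversing direction at either end to ping-pong.
; The kick event plays a wheel-kick montage and calls KICKfinished on completion or interruption.
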(event `fucking kick!!!!`
  (`KismetSystemLibrary.PrintString` "KICKING YOU KICKING YOU KICKING YOU")
  (`|PlayMontage` (`self.Mesh`) "/Game/CloseCombatAnimSet/Animations/InPlace/Attacks/NinjaWheelKick_Montage.NinjaWheelKick_Montage"
    (:`OnCompleted`
      _)
    (:`OnInterrupted`
      _))
  (`self.KICKfinished`))

(event `self.ReceiveBeginPlay`
  (set `self.OriginalMaterial` (`PrimitiveComponent.GetMaterial` (`self.Mesh`) 0)))

(event `GetAggro`
  (`PrimitiveComponent.SetMaterial` (`self.Mesh`) 0 "/AnimationSharing/AnimSharingRed.AnimSharingRed")
  (set `self.Aggroed` true))

(event `LoseAggro`
  (`PrimitiveComponent.SetMaterial` (`self.Mesh`) 0 (`self.OriginalMaterial`))
  (set `self.Aggroed` false))

(event `Begin_Investigate`
  (`PrimitiveComponent.SetMaterial` (`self.Mesh`) 0 "/AnimationSharing/AnimSharingGreen.AnimSharingGreen")
  (set `self.Investigating` true))

(event `Quit_Investigate`
  (`PrimitiveComponent.SetMaterial` (`self.Mesh`) 0 (`self.OriginalMaterial`))
  (set `self.Investigating` false))

(fn `GetNextPatrolPointLocation`
  (returns (ReturnValue :type "Vector Structure"))
  (`/Engine/EditorBlueprintResources/StandardMacros.IsValid` (`self.PatrolRoute`)
    (:`Is Valid`
      ; if greater than spline points or less than 0 return true
      (set `self.Point Index` (+ (`self.Point Index`) (`self.PatrolRouteDirection`))) ; update next point
      (if (or (>= (`self.Point Index`) (- (`SplineComponent.GetNumberOfSplinePoints` (`/Game/AI_Blueprints/BP_PatrolRoute.Spline` (`self.PatrolRoute`))) 1)) (<= (`self.Point Index`) 0))
        ; flip the direction
        (set `self.PatrolRouteDirection` (* (`self.PatrolRouteDirection`) -1)))
      (return (`SplineComponent.GetLocationAtSplinePoint` (`/Game/AI_Blueprints/BP_PatrolRoute.Spline` (`self.PatrolRoute`)) (`self.Point Index`) "World")))
    (:`Is Not Valid`
      (`KismetSystemLibrary.PrintText` "I don't have a tahrgoht"))))

(fn `UserConstructionScript`)