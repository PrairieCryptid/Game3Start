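; Enemy spawner that populates the level with randomized AI characters when play begins.
; It finds every BP_enemspawnPoint actor and gives each a 90% chance to spawn a BP_AiMoveTo at its transform.
; Each spawn gets random materials on two slots, then a random skeletal mesh from an array.
; Its name label shows a random index from the Name array as a number, rather than the entry itself.
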(event `self.ReceiveBeginPlay`
  (bind _outitem (`KismetArrayLibrary.Array_Random` (`self.MaterialArray`)))
  (`KismetSystemLibrary.PrintString` "Spawner Online")
  (bind _outactors (`GameplayStatics.GetAllActorsOfClass` "/Game/Blueprints/BP_enemspawnPoint.BP_enemspawnPoint_C"))
  (for _array_element _outactors
    (if (`KismetMathLibrary.RandomBoolWithWeight` 0.9)
      (bind _returnvalue (`|SpawnActorFromClass` "/Game/AI_Blueprints/BP_AiMoveTo.BP_AiMoveTo_C" (`self.GetTransform` _array_element) "Undefined" "MultiplyWithRoot" null null))
      (`TextRenderComponent.K2_SetText` (`/Game/AI_Blueprints/BP_AiMoveTo.AINameNext` _returnvalue) (`KismetTextLibrary.Conv_IntToText` (`.OutIndex` (`KismetArrayLibrary.Array_Random` (`self.Name`)))))
      (bind _mesh (`Character.Mesh` _returnvalue))
      (`PrimitiveComponent.SetMaterial` _mesh 0 _outitem)
      (`PrimitiveComponent.SetMaterial` _mesh 1 _outitem)
      (`SkeletalMeshComponent.SetSkeletalMeshAsset` _mesh (`KismetArrayLibrary.Array_Random` (`self.MeshArray`))))))

(fn `UserConstructionScript`)