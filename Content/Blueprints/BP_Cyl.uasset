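; BP_Cyl is a machine gun pickup that can be attached to a skeletal mesh and dropped.
; Pickup prints a debug message, snaps the gun to the IK_hand_r socket and turns off MGBody collision.
; Drop detaches it in world space and enables physics on MGBody, again after a short delay, but sets collision to NoCollision and never restores it.
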(event `self.Pickup`
  (params (SkeletalMesh :type "SkeletalMeshComponent Object Reference"))
  ; the motherfucking FUTURE
  (`KismetSystemLibrary.PrintText` (`|FormatText` "{name} is getting picked up, and attatched to {mesh},  soldier!" "MachineGun" SkeletalMesh) true true (struct :`R` 1.0 :`B` 0.887938 :`A` 1.0))
  (`self.K2_AttachToComponent` SkeletalMesh "IK_hand_r" "SnapToTarget" "SnapToTarget" "SnapToTarget")
  (`PrimitiveComponent.SetCollisionEnabled` (`self.MGBody`) "NoCollision"))

(event `self.Drop`
  (bind _mgbody (`self.MGBody`))
  (`self.K2_DetachFromActor` "KeepWorld" "KeepWorld" "KeepWorld")
  (`PrimitiveComponent.SetSimulatePhysics` _mgbody true)
  (`PrimitiveComponent.SetCollisionEnabled` _mgbody "NoCollision")
  (`KismetSystemLibrary.Delay` 0.2)
  (`PrimitiveComponent.SetSimulatePhysics` _mgbody true))

(fn `UserConstructionScript`)